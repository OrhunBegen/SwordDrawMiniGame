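; Samurai duelist for a reaction-based draw game, built on a Paper2D sprite and driven by the phase in GM_Duel.
; Attack allows one press until Reset: during Wait it shows a cross and locks out; during Draw it ends the phase.
; A winning press plays a timeline lunge that swaps to the attack sprite and reports success, flagging player control.
; Timelines also handle the slide-in on start and reset; Defeated swaps the sprite.
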(event Custom|Slide%20in
  (bind _papersprite (Variables|Default|GetPaperSprite))
  (Components|Timeline|SetPlayRate (Variables|Default|GetSlideInAnim) 2.0)
  (bind _alpha (Timeline|SlideInAnim PlayFromStart)
    (:Update
      (Transformation|SetRelativeLocation _papersprite (Math|Vector|Lerp(Vector) (Variables|Default|GetStartPoint) (Variables|Default|GetSprite%20Default%20Position) _alpha) false false)
      (Rendering|SetTranslucentSortPriority _papersprite 1)
      (Rendering|Material|SetMaterial _papersprite 0 "/Paper2D/TranslucentUnlitSpriteMaterial.TranslucentUnlitSpriteMaterial"))))

(event Custom|Attack
  (bind _papersprite (Variables|Default|GetPaperSprite))
  (if (not (Variables|Default|GetPressedDraw))
    (switch Utilities|FlowControl|Switch|SwitchonE_Phase (Variables|/Game/GameMode/GM_Duel.GM_Duel_C|GetEPhase (Variables|Default|GetGameMode))
      (:NewEnumerator1
        (CallFunction|SetCrossVisibility true)
        (Variables|Default|SetPressedDraw true))
      (:NewEnumerator2
        (Variables|Default|SetPressedDraw true)
        (Default|SetGameModeFinished (Variables|Default|GetGameMode))
        (Components|Timeline|SetPlayRate (Variables|Default|GetAttackAnim) 2e+01)
        (bind _alpha (Timeline|AttackAnim PlayFromStart)
          (:Update
            (Transformation|SetRelativeLocationAndRotation (Variables|Default|GetPaperSprite) (Math|Vector|Lerp(Vector) (Variables|Default|GetRelative%20Location) (Variables|/Script/Engine.SceneComponent|GetRelativeLocation (Variables|Default|GetScene)) _alpha) "0, 0, 0" false false))
          (:SetSprite
            (Rendering|Components|Sprite|SetSprite _papersprite (Variables|Default|GetAttackState))
            (Rendering|SetTranslucentSortPriority _papersprite 1)
            (Rendering|Material|SetMaterial _papersprite 0 "/Paper2D/TranslucentUnlitSpriteMaterial.TranslucentUnlitSpriteMaterial")
            (Default|AttackedSuccessfully (Variables|Default|GetGameMode) (Pawn|IsPlayerControlled))))))))

(event Custom|Defeated
  (Rendering|Components|Sprite|SetSprite (Variables|Default|GetPaperSprite) (Variables|Default|GetDefeatedState)))

(event EventBeginPlay
  (bind _asgm_duel (Utilities|Casting|CastToGM_Duel (Game|GetGameMode)))
  (Variables|Default|SetGameMode _asgm_duel)
  (Variables|Default|SetSprite%20Default%20Position (Variables|/Script/Engine.SceneComponent|GetRelativeLocation (Variables|Default|GetPaperSprite)))
  (CallFunction|Slidein)
  (CallFunction|SetCrossVisibility false))

(fn ConstructionScript)

(fn SetCrossVisibility
  (params (bNewVisibility :type Boolean))
  (Rendering|SetVisibility (Variables|Default|Getcross) bNewVisibility false))

(fn Reset
  (Rendering|Components|Sprite|SetSprite (Variables|Default|GetPaperSprite) (Variables|Default|GetIdleState))
  (Variables|Default|SetPressedDraw false)
  (CallFunction|Slidein))