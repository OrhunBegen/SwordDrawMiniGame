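; Game mode for a samurai reaction duel between the player and an AI, run as an Intro, Wait, Draw, Finished phase machine.
; Tick ends Intro after a start time, then a random delay opens Draw, fires DrawPhaseStarted and shows the exclamation cue.
; AttackedSuccessfully defeats the loser, hides the cue and starts a restart timer.
; Reset restores Intro and both fighters, while SetGameModeFinished sets the Finished phase.
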(event EventBeginPlay
  (bind _returnvalue (Actor|GetActorOfClass "/Game/Blueprints/BP_Explenations.BP_Explenations_C"))
  (Variables|Default|SetExclamRef _returnvalue)
  (bind _returnvalue_2 (Actor|GetActorOfClass "/Game/Blueprints/BP_Samurai_Player.BP_Samurai_Player_C"))
  (Variables|Default|SetSamuraiPlayer _returnvalue_2)
  (bind _returnvalue_3 (Actor|GetActorOfClass "/Game/Blueprints/BP_CustomAi.BP_CustomAi_C"))
  (Variables|Default|SetSamuraiAi _returnvalue_3))

(event EventTick
  (params (DeltaSeconds :type Float%20%28single-precision%29))
  (Variables|Default|SetElapsedTime (+ DeltaSeconds (Variables|Default|GetElapsedTime)))
  (switch Utilities|FlowControl|Switch|SwitchonE_Phase (Variables|Default|GetEPhase)
    (:NewEnumerator0
      (if (>= (Variables|Default|GetElapsedTime) (Variables|Default|GetRoundStartTime))
        (Variables|Default|SetEPhase "NewEnumerator1")
        (Utilities|FlowControl|Delay (Math|Random|RandomFloatinRange (Variables|Default|GetMin) (Variables|Default|GetMax)))
        (Variables|Default|SetEPhase "NewEnumerator2")
        (Default|CallDrawPhaseStarted)
        (Utilities|IsValid (Variables|Default|GetExclamRef)
          (:Is%20Valid
            (Default|SetVisibility (Variables|Default|GetExclamRef) true))
          (:Is%20Not%20Valid
            (Development|PrintString "Error")))))))

(fn ConstructionScript)

(fn SetGameModeFinished
  (Variables|Default|SetEPhase "NewEnumerator3"))

(fn AttackedSuccessfully
  (params (IsPlayer :type Boolean))
  (if IsPlayer
    (Default|Defeated (Variables|Default|GetSamuraiAi))
    (else
      (Default|Defeated (Variables|Default|GetSamuraiPlayer))))
  (Utilities|IsValid (Variables|Default|GetExclamRef)
    (:Is%20Valid
      (Default|SetVisibility (Variables|Default|GetExclamRef) false)
      (Utilities|Time|SetTimerbyEvent (EventDispatchers|CreateEvent :!event Reset) (Variables|Default|GetRestartDelay)))))

(fn Reset
  (Variables|Default|SetEPhase "NewEnumerator0")
  (Default|Reset (Variables|Default|GetSamuraiAi))
  (Default|Reset (Variables|Default|GetSamuraiPlayer)))